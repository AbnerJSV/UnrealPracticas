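; BP_Enemy2 is a child enemy Blueprint that trades damage with the top-down player character through its Interact function.
; Interact casts the passed object to BP_TopDownCharacter and applies DamageAmount to that character's health component.
; The enemy then takes fixed damage on its own health component and destroys itself when TakeDamage returns true, logging each step with debug prints.
; Overlap handling defers to the parent class.
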(event EventBeginPlay
  (|CallParentFunction) ; This node is disabled and will not be called.\nDrag off pins to build functionality.
)

(event Collision|EventActorBeginOverlap
  (params (OtherActor :type Actor%20Object%20Reference))
  (|CallParentFunction OtherActor))

(event EventTick
  (params (DeltaSeconds :type Float%20%28single-precision%29))
  (|CallParentFunction DeltaSeconds) ; This node is disabled and will not be called.\nDrag off pins to build functionality.
)

(fn ConstructionScript
  (|CallParentFunction))

(fn Interact
  (params (Object :type Object%20Object%20Reference))
  (Development|PrintString "Enemy: Le hice daño al jugador")
  (bind _asbp_top_down_character (Utilities|Casting|CastToBP_TopDownCharacter Object))
  (bind _isdead (Default|TakeDamage (Variables|/Game/TopDown/Blueprints/BP_TopDownCharacter.BP_TopDownCharacter_C|GetBPC_HealthComponent _asbp_top_down_character) (Variables|Default|GetDamageAmount)))
  (if _isdead
    (Development|PrintString "Enemy: Player Muerto"))
  (Development|PrintString "Enemy: Recibi Daño")
  (bind _isdead_2 (Default|TakeDamage (Variables|Default|GetBPC_HealthComponent) 25.0))
  (if _isdead_2
    (Actor|DestroyActor)))