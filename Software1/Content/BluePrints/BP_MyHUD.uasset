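; BP_MyHUD is a HUD Blueprint that shows the game info widget and manages the shop screen.
; On BeginPlay it creates WBP_GameInfo and adds it to the viewport.
; OpenShop creates a new WBP_Shop, stores it, pauses the game and displays it.
; CloseShop unpauses the game and removes that stored shop widget from its parent.
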(event EventBeginPlay
  (bind _returnvalue (UserInterface|CreateWidget "/Game/BluePrints/WBP_GameInfo.WBP_GameInfo_C"))
  (UserInterface|Viewport|AddtoViewport _returnvalue 0))

(event EventTick
  (params (DeltaSeconds :type Float%20%28single-precision%29)))

(event Collision|EventActorBeginOverlap
  (params (OtherActor :type Actor%20Object%20Reference)))

(fn ConstructionScript)

(fn OpenShop
  (bind _returnvalue (UserInterface|CreateWidget "/Game/BluePrints/WBP_Shop.WBP_Shop_C"))
  (bind _output_get (Variables|Default|SetShopReference _returnvalue))
  (Game|SetGamePaused true)
  (UserInterface|Viewport|AddtoViewport _output_get 0))

(fn CloseShop
  (Game|SetGamePaused false)
  (Widget|RemovefromParent (Variables|Default|GetShopReference)))