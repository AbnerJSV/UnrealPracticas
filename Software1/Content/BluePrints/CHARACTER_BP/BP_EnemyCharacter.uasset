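; BP_EnemyCharacter is an enemy that chases the player and deals damage on overlap.
; A chase event runs AIMoveTo toward the player from BeginPlay, re-triggering one second after each successful move and also after hitting the player.
; It reports spawn and death to BP_RandomSpawn_Enemy, found via GetActorOfClass, and destroys itself when its health component signals death.
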(event Death(BPC_HealthComponent)
  (bind _returnvalue (Actor|GetActorOfClass "/Game/BluePrints/Manager/BP_RandomSpawn_Enemy.BP_RandomSpawn_Enemy_C"))
  (Default|EnemyDeathEvent _returnvalue)
  (Actor|DestroyActor))

(event Custom|Chase_Event
  (AI|AIMoveTo self "0, 0, 0" (Game|GetPlayerCharacter 0) 5.0 false
    (:OnSuccess
      (Utilities|FlowControl|Delay 1.0)
      (CallFunction|ChaseEvent))))

(event EventBeginPlay
  (CallFunction|ChaseEvent)
  (bind _returnvalue (Actor|GetActorOfClass "/Game/BluePrints/Manager/BP_RandomSpawn_Enemy.BP_RandomSpawn_Enemy_C"))
  (Default|EnemyAliveEvent _returnvalue))

(event Collision|EventActorBeginOverlap
  (params (OtherActor :type Actor%20Object%20Reference))
  (bind _asbp_top_down_character (Utilities|Casting|CastToBP_TopDownCharacter OtherActor))
  (Default|Damage (Variables|/Game/TopDown/Blueprints/BP_TopDownCharacter.BP_TopDownCharacter_C|GetBPC_HealthComponent _asbp_top_down_character) (Variables|Default|GetDamageAmount))
  (CallFunction|ChaseEvent))

(event EventTick
  (params (DeltaSeconds :type Float%20%28single-precision%29)))

(fn ConstructionScript)