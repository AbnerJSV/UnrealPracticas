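; HUD Blueprint that swaps on-screen widgets to match the game state: Game Start, Round, Rest, Victory or Game Over.
; Round and Rest show game info with a refreshed inventory, while every state except Round opens a Continue widget, pausing the game outside Rest.
; Closing Continue unpauses and tells BP_GameManager to end the current state.
; Separate functions open and close the shop, pausing the game while it is shown.
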(event Custom|ActualEstate_Event
  (params (State :type E_GameState%20Enum :default "NewEnumerator0"))
  (switch Utilities|FlowControl|Switch|SwitchonE_GameState State
    (:NewEnumerator0
      (CallFunction|GameStartEvent))
    (:NewEnumerator1
      (CallFunction|RoundEvent))
    (:NewEnumerator2
      (CallFunction|RestEvent))
    (:NewEnumerator3
      (CallFunction|VictoryEvent))
    (:NewEnumerator4
      (CallFunction|GameOverEvent))))

(event Custom|GameStart_Event
  (CallFunction|OpenContinueWidget true))

(event Custom|Round_Event
  (CallFunction|EndActualStateEvent)
  (bind _returnvalue (UserInterface|CreateWidget "/Game/BluePrints/HUD/WBP_GameInfo.WBP_GameInfo_C"))
  (UserInterface|Viewport|AddtoViewport _returnvalue 0)
  (CallFunction|ReloadInventoryEvent))

(event Custom|Rest_Event
  (CallFunction|EndActualStateEvent)
  (CallFunction|OpenContinueWidget false)
  (bind _returnvalue (UserInterface|CreateWidget "/Game/BluePrints/HUD/WBP_GameInfo.WBP_GameInfo_C"))
  (UserInterface|Viewport|AddtoViewport _returnvalue 0)
  (CallFunction|ReloadInventoryEvent))

(event Custom|Victory_Event
  (CallFunction|EndActualStateEvent)
  (CallFunction|OpenContinueWidget true))

(event Custom|GameOver_Event
  (CallFunction|EndActualStateEvent)
  (CallFunction|OpenContinueWidget true))

(event Custom|EndActualState_Event
  (Viewport|RemoveAllWidgets))

(event Custom|ReloadInventory_Event
  (bind _foundwidgets (Widget|GetAllWidgetsOfClass "/Game/BluePrints/HUD/WBP_GameInfo.WBP_GameInfo_C" true))
  (Default|RefreshInventory _foundwidgets))

(event EventBeginPlay)

(event EventTick
  (params (DeltaSeconds :type Float%20%28single-precision%29)))

(event Collision|EventActorBeginOverlap
  (params (OtherActor :type Actor%20Object%20Reference)))

(fn ConstructionScript)

(fn OpenShop
  (bind _returnvalue (UserInterface|CreateWidget "/Game/BluePrints/HUD/WBP_Shop.WBP_Shop_C"))
  (bind _output_get (Variables|Default|SetShopReference _returnvalue))
  (Game|SetGamePaused true)
  (UserInterface|Viewport|AddtoViewport _output_get 0))

(fn CloseShop
  (Game|SetGamePaused false)
  (Widget|RemovefromParent (Variables|Default|GetShopReference)))

(fn OpenContinueWidget
  (params (Paused :type Boolean))
  (bind _returnvalue (UserInterface|CreateWidget "/Game/BluePrints/HUD/WBP_Continue.WBP_Continue_C" (Game|GetPlayerController 0)))
  (bind _output_get (Variables|Default|SetContinueReference _returnvalue))
  (UserInterface|Viewport|AddtoViewport _output_get 0)
  (Game|SetGamePaused Paused))

(fn CloseContinueWidget
  (Game|SetGamePaused false)
  (Widget|RemovefromParent (Variables|Default|GetContinueReference))
  (bind _returnvalue (Actor|GetActorOfClass "/Game/BluePrints/Manager/BP_GameManager.BP_GameManager_C"))
  (Default|EndActualStateEvent _returnvalue false))