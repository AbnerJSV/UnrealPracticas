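; BP_Chest is an interactable chest that gives the top-down player character one random reward.
; Interact checks CanOpen, picks a random entry from Rewards, adds it to the inventory component of the BP_TopDownCharacter found by class, then clears CanOpen so the chest pays out only once.
; The Object passed to Interact is unused, and the event graph holds only disabled default events.
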(event EventBeginPlay
  (|CallParentFunction) ; This node is disabled and will not be called.\nDrag off pins to build functionality.
)

(event Collision|EventActorBeginOverlap
  (params (OtherActor :type Actor%20Object%20Reference))
  (|CallParentFunction OtherActor) ; This node is disabled and will not be called.\nDrag off pins to build functionality.
)

(event EventTick
  (params (DeltaSeconds :type Float%20%28single-precision%29))
  (|CallParentFunction DeltaSeconds) ; This node is disabled and will not be called.\nDrag off pins to build functionality.
)

(fn ConstructionScript)

(fn Interact
  (params (Object :type Object%20Object%20Reference))
  (if (Variables|Default|GetCanOpen)
    (bind _returnvalue (Actor|GetActorOfClass "/Game/TopDown/Blueprints/BP_TopDownCharacter.BP_TopDownCharacter_C"))
    (Default|AddReward (Variables|/Game/TopDown/Blueprints/BP_TopDownCharacter.BP_TopDownCharacter_C|GetBPC_InventoryComponent _returnvalue) (.OutItem (Utilities|Array|Random (Variables|Default|GetRewards))))
    (Variables|Default|SetCanOpen false)))