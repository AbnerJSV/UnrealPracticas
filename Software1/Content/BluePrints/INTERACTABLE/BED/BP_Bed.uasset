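; BP_Bed is an interactable bed that heals the player's top-down character when used.
; Interact prints a Spanish debug message, casts the passed object to BP_TopDownCharacter, then calls Heal on its BPCHealthComponent with HealAmount.
; Objects that fail the cast receive no healing.
; Overlap only forwards to the parent class, and BeginPlay and Tick are disabled.
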(event EventBeginPlay
  (|CallParentFunction) ; This node is disabled and will not be called.\nDrag off pins to build functionality.
)

(event Collision|EventActorBeginOverlap
  (params (OtherActor :type Actor%20Object%20Reference))
  (|CallParentFunction OtherActor))

(event EventTick
  (params (DeltaSeconds :type Float%20%28single-precision%29))
  (|CallParentFunction DeltaSeconds) ; This node is disabled and will not be called.\nDrag off pins to build functionality.
)

(fn ConstructionScript
  (|CallParentFunction))

(fn Interact
  (params (Object :type Object%20Object%20Reference))
  (Development|PrintString "Cama: Cura vida")
  (bind _asbp_top_down_character (Utilities|Casting|CastToBP_TopDownCharacter Object))
  (Default|Heal (Variables|/Game/TopDown/Blueprints/BP_TopDownCharacter.BP_TopDownCharacter_C|GetBPC_HealthComponent _asbp_top_down_character) (Variables|Default|GetHealAmount)))