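; BP_Projectile is a player attack projectile that flies toward a target location and damages enemy characters it overlaps.
; At BeginPlay it fixes its direction and copies Damage and Speed from the top-down character's BPCAttackComponent.
; Tick moves it without sweep and destroys it near the target location.
; Overlaps apply damage through the enemy's BPCHealthComponent without destroying the projectile, so it can pass through enemies.
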(event EventBeginPlay
  (Variables|Default|SetDirection (Math|Vector|Normalize (- (Variables|Default|GetTargetLocation) (Transformation|GetActorLocation))))
  (bind _returnvalue (Actor|GetActorOfClass "/Game/TopDown/Blueprints/BP_TopDownCharacter.BP_TopDownCharacter_C"))
  (Variables|Default|SetDamage (Variables|/Game/BluePrints/COMPONENT/BPC_AttackComponent.BPC_AttackComponent_C|GetDamage (Variables|/Game/TopDown/Blueprints/BP_TopDownCharacter.BP_TopDownCharacter_C|GetBPC_AttackComponent _returnvalue)))
  (Variables|Default|SetSpeed (Variables|/Game/BluePrints/COMPONENT/BPC_AttackComponent.BPC_AttackComponent_C|GetSpeed (Variables|/Game/TopDown/Blueprints/BP_TopDownCharacter.BP_TopDownCharacter_C|GetBPC_AttackComponent _returnvalue))))

(event Collision|EventActorBeginOverlap
  (params (OtherActor :type Actor%20Object%20Reference))
  (bind _asbp_enemy_character (Utilities|Casting|CastToBP_EnemyCharacter OtherActor))
  (Default|Damage (Variables|/Game/BluePrints/CHARACTER_BP/BP_EnemyCharacter.BP_EnemyCharacter_C|GetBPC_HealthComponent _asbp_enemy_character) (Variables|Default|GetDamage)))

(event EventTick
  (params (DeltaSeconds :type Float%20%28single-precision%29))
  (bind _returnvalue (Transformation|GetActorLocation))
  (Transformation|SetActorLocation (+ _returnvalue (* (Variables|Default|GetDirection) (Variables|Default|GetSpeed) DeltaSeconds)) false false)
  (if (< (Math|Vector|Distance(Vector) _returnvalue (Variables|Default|GetTargetLocation)) 1e+02)
    (Actor|DestroyActor)))

(fn ConstructionScript
  (|CallParentFunction))