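; BPC_AttackComponent is a component that holds Damage and Speed stats and applies upgrades to them.
; On BeginPlay it caches the starting values as BaseDamage and BaseSpeed.
; DamageUpgrade and SpeedUpgrade recompute each stat as the given amount times its per-upgrade increment plus the cached base, so repeated calls replace the bonus instead of stacking it.
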(event EventBeginPlay
  (Variables|Default|SetBaseDamage (Variables|Default|GetDamage))
  (Variables|Default|SetBaseSpeed (Variables|Default|GetSpeed)))

(event EventTick
  (params (DeltaSeconds :type Float%20%28single-precision%29)))

(fn DamageUpgrade
  (params (AmountOfDamage :type Float%20%28double-precision%29))
  (Variables|Default|SetDamage (+ (* AmountOfDamage (Variables|Default|GetUpgradeDamageAmount)) (Variables|Default|GetBaseDamage))))

(fn SpeedUpgrade
  (params (AmountOfMoveSpeed :type Float%20%28double-precision%29))
  (Variables|Default|SetSpeed (+ (* AmountOfMoveSpeed (Variables|Default|GetUpgradeSpeedAmount)) (Variables|Default|GetBaseSpeed))))