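; Health component that tracks an actor's current and maximum health, handling damage, healing and max health upgrades.
; BeginPlay fills current health and stores the starting maximum as a base value.
; Damage clamps health at zero, fires CallDeath and returns whether health ran out, while Heal caps at the maximum.
; HealthUpgrade recomputes the maximum from that base plus an upgrade count times a per-upgrade amount, leaving current health unchanged.
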(event EventBeginPlay
  (Variables|Default|SetCurrentHealth (Variables|Default|GetMaxHealth))
  (Variables|Default|SetBaseHealth (Variables|Default|GetMaxHealth)))

(event EventTick
  (params (DeltaSeconds :type Float%20%28single-precision%29)))

(fn Damage
  (params (DamageAmount :type Float%20%28double-precision%29))
  (Variables|Default|SetCurrentHealth (- (Variables|Default|GetCurrentHealth) DamageAmount))
  (if (<= (Variables|Default|GetCurrentHealth) 0.0)
    (Variables|Default|SetCurrentHealth 0.0)
    (Default|CallDeath))
  (return (<= (Variables|Default|GetCurrentHealth) 0.0)))

(fn Heal
  (params (HealAmount :type Float%20%28double-precision%29))
  (if (>= (+ HealAmount (Variables|Default|GetCurrentHealth)) (Variables|Default|GetMaxHealth))
    (Variables|Default|SetCurrentHealth (Variables|Default|GetMaxHealth))
    (else
      (Variables|Default|SetCurrentHealth (+ HealAmount (Variables|Default|GetCurrentHealth))))))

(fn HealthUpgrade
  (params (AmountOfMaxHealth :type Float%20%28double-precision%29))
  (Variables|Default|SetMaxHealth (+ (* AmountOfMaxHealth (Variables|Default|GetUpgradeHealthAmount)) (Variables|Default|GetBaseHealth))))