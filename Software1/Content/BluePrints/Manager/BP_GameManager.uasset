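; BP_GameManager runs the game's phase state machine: Game Start, Round, Rest, Victory and Game Over.
; Ending a state advances it, with the last round leading to Victory, and each entered state is reported to the HUD.
; Rounds clear chests and start enemy and pickup spawners, while rests start chest spawners.
; Game Over reboots the enemy spawner; Game Start and Victory handlers are empty.
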(event Custom|ActualState_Event
  (CallFunction|MyHUD)
  (switch Utilities|FlowControl|Switch|SwitchonE_GameState (Variables|Default|GetCurrentState)
    (:NewEnumerator0
      (CallFunction|GameStartEvent))
    (:NewEnumerator1
      (CallFunction|RoundEvent))
    (:NewEnumerator2
      (CallFunction|RestEvent))
    (:NewEnumerator3
      (CallFunction|VictoryEvent))
    (:NewEnumerator4
      (CallFunction|GameOverEvent))))

(event Custom|GameStart_Event)

(event Custom|Round_Event
  (Utilities|FlowControl|Sequence
    (:then_0
      (bind _outactors (Actor|GetAllActorsOfClass "/Game/BluePrints/INTERACTABLE/CHEST/BP_Chest.BP_Chest_C"))
      (Actor|DestroyActor _outactors))
    (:then_1
      (bind _returnvalue (Actor|GetActorOfClass "/Game/BluePrints/Manager/BP_RandomSpawn_Enemy.BP_RandomSpawn_Enemy_C"))
      (Default|StartEnemySpawnerEvent _returnvalue))
    (:then_2
      (bind _returnvalue_2 (Actor|GetActorOfClass "/Game/BluePrints/Manager/BP_RandomSpawn_Pickup.BP_RandomSpawn_Pickup_C"))
      (Default|StartPickupSpawnerEvent _returnvalue_2))))

(event Custom|Rest_Event
  (bind _outactors (Actor|GetAllActorsOfClass "/Game/BluePrints/Manager/BP_ChestSpawner.BP_ChestSpawner_C"))
  (Default|StartChestEvent _outactors))

(event Custom|Victory_Event)

(event Custom|GameOver_Event
  (Variables|Default|SetCurrentState "NewEnumerator4")
  (bind _returnvalue (Actor|GetActorOfClass "/Game/BluePrints/Manager/BP_RandomSpawn_Enemy.BP_RandomSpawn_Enemy_C"))
  (Default|RebootEnemySpawnerEvent _returnvalue))

(event Custom|EndActualState_Event
  (params (IsLastRound :type Boolean))
  (switch Utilities|FlowControl|Switch|SwitchonE_GameState (Variables|Default|GetCurrentState)
    (:NewEnumerator0
      (Variables|Default|SetCurrentState "NewEnumerator1"))
    (:NewEnumerator1
      (if IsLastRound
        (Variables|Default|SetCurrentState "NewEnumerator3")
        (else
          (Variables|Default|SetCurrentState "NewEnumerator2"))))
    (:NewEnumerator2
      (Variables|Default|SetCurrentState "NewEnumerator1"))
    (:NewEnumerator3
      (Variables|Default|SetCurrentState "NewEnumerator0"))
    (:NewEnumerator4
      (Variables|Default|SetCurrentState "NewEnumerator0")))
  (CallFunction|ActualStateEvent))

(event EventBeginPlay
  (Variables|Default|SetCurrentState "NewEnumerator0")
  (Utilities|FlowControl|DelayUntilNextTick)
  (CallFunction|ActualStateEvent))

(event EventTick
  (params (DeltaSeconds :type Float%20%28single-precision%29)))

(fn ConstructionScript)

(fn MyHUD
  (bind _returnvalue (Actor|GetActorOfClass "/Game/BluePrints/HUD/HBP_MyHUD.HBP_MyHUD_C"))
  (Default|ActualEstateEvent _returnvalue (Variables|Default|GetCurrentState)))