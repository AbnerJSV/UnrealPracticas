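; BP_RandomSpawn_Enemy is a round-based enemy spawner that builds on a parent spawn Blueprint.
; A looping timer calls the inherited spawn event under the alive cap, stopping once the round quota is spawned.
; Alive and death events track counts; a cleared round raises the quota and tells BP_GameManager whether the final round was reached.
; A reboot event destroys all enemies and restores the original counters.
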(event Custom|StartEnemySpawner_Event
  (Math|Integer|IncrementInt (Variables|Default|GetRoundActive)
    (:%20%20
      (bind _returnvalue (Utilities|Time|SetTimerbyEvent (delegate Custom|SpawnEnemy_Event) (Variables|Default|GetSpawnInterval) true))
      (Variables|Default|SetTimerByEvent _returnvalue))))

(event Custom|Spawn_Event
  (|CallParentFunction))

(event Custom|EndEnemySpawner_Event
  (if (== (Variables|Default|GetEnemiesPerRound) (Variables|Default|GetEnemiesSpawned))
    (if (== (Variables|Default|GetEnemiesAlive) 0)
      (Variables|Default|SetEnemiesSpawned 0)
      (Variables|Default|SetEnemiesAlive 0)
      (Variables|Default|SetEnemiesPerRound (+ (Variables|Default|GetEnemiesPerRound) (Variables|Default|GetIncreaseEnemiesPerRound)))
      (bind _returnvalue (Actor|GetActorOfClass "/Game/BluePrints/Manager/BP_GameManager.BP_GameManager_C"))
      (Default|EndActualStateEvent _returnvalue (== (Variables|Default|GetRoundActive) (Variables|Default|GetMaxRound))))))

(event Custom|EnemyDeath_Event
  (Math|Integer|DecrementInt (Variables|Default|GetEnemiesAlive)
    (:%20%20
      (CallFunction|EndEnemySpawnerEvent))))

(event Custom|EnemyAlive_Event
  (Math|Integer|IncrementInt (Variables|Default|GetEnemiesSpawned)
    (:%20%20
      (Math|Integer|IncrementInt (Variables|Default|GetEnemiesAlive)))))

(event Custom|RebootEnemySpawner_Event
  (bind _outactors (Actor|GetAllActorsOfClass "/Game/BluePrints/CHARACTER_BP/BP_EnemyCharacter.BP_EnemyCharacter_C"))
  (for _array_element _outactors
    (Actor|DestroyActor _array_element))
  (Variables|Default|SetEnemiesSpawned 0)
  (Variables|Default|SetEnemiesAlive 0)
  (Variables|Default|SetRoundActive 0)
  (Variables|Default|SetEnemiesPerRound (Variables|Default|GetEnemiesPerRoundOriginal)))

(event Custom|SpawnEnemy_Event
  (if (> (Variables|Default|GetMaxAliveEnemies) (Variables|Default|GetEnemiesAlive))
    (if (< (Variables|Default|GetEnemiesSpawned) (Variables|Default|GetEnemiesPerRound))
      (CallFunction|SpawnEvent)
      (else
        (Utilities|Time|ClearandInvalidateTimerbyHandle (Variables|Default|GetTimerByEvent))))))

(event EventBeginPlay
  (Variables|Default|SetEnemiesPerRoundOriginal (Variables|Default|GetEnemiesPerRound)))

(fn ConstructionScript
  (|CallParentFunction))