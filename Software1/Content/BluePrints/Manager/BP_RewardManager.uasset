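; BP_RewardManager turns the rewards in the player's inventory into stat upgrades.
; NewReward refreshes the HUD inventory, then resets and recounts rewards by type: max health, damage, move speed and projectile speed.
; It passes the totals to the character and its health and attack components.
; The projectile speed upgrade receives the move speed count, leaving its own count unused.
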(event Custom|NewReward_Event
  (Utilities|FlowControl|Sequence
    (:then_0
      (bind _returnvalue (Actor|GetActorOfClass "/Game/BluePrints/HUD/HBP_MyHUD.HBP_MyHUD_C"))
      (Default|ReloadInventoryEvent _returnvalue))
    (:then_1
      (CallFunction|CountRewardsEvent))))

(event Custom|ActivateReward_Event
  (Utilities|FlowControl|Sequence
    (:then_0
      (CallFunction|MaxHealthEvent))
    (:then_1
      (CallFunction|DamageEvent))
    (:then_2
      (CallFunction|MoveSpeedEvent))
    (:then_3
      (CallFunction|ProjectileSpeedEvent))))

(event Custom|CountRewards_Event
  (bind _asbp_top_down_character (Utilities|Casting|CastToBP_TopDownCharacter (Game|GetPlayerCharacter 0)))
  (CallFunction|SetAmountstoZero)
  (for _array_element (Variables|/Game/BluePrints/COMPONENT/BPC_InventoryComponent.BPC_InventoryComponent_C|GetRewards (Variables|/Game/TopDown/Blueprints/BP_TopDownCharacter.BP_TopDownCharacter_C|GetBPC_InventoryComponent _asbp_top_down_character))
    (switch Utilities|FlowControl|Switch|SwitchonE_RewardType (Variables|/Game/BluePrints/Inventario/PDA_Reward.PDA_Reward_C|GetRewardType _array_element)
      (:NewEnumerator0
        (Math|Float|IncrementFloat (Variables|Default|GetAmountOfMaxHealth)))
      (:NewEnumerator1
        (Math|Float|IncrementFloat (Variables|Default|GetAmountOfDamage)))
      (:NewEnumerator2
        (Math|Float|IncrementFloat (Variables|Default|GetAmountOfMoveSpeed)))
      (:NewEnumerator3
        (Math|Float|IncrementFloat (Variables|Default|GetAmountOfProjectileSpeed)))))
  (CallFunction|ActivateRewardEvent))

(event Custom|MaxHealth_Event
  (bind _asbp_top_down_character (Utilities|Casting|CastToBP_TopDownCharacter (Game|GetPlayerCharacter 0)))
  (Default|HealthUpgrade (Variables|/Game/TopDown/Blueprints/BP_TopDownCharacter.BP_TopDownCharacter_C|GetBPC_HealthComponent _asbp_top_down_character) (Variables|Default|GetAmountOfMaxHealth)))

(event Custom|Damage_Event
  (bind _asbp_top_down_character (Utilities|Casting|CastToBP_TopDownCharacter (Game|GetPlayerCharacter 0)))
  (Default|DamageUpgrade (Variables|/Game/TopDown/Blueprints/BP_TopDownCharacter.BP_TopDownCharacter_C|GetBPC_AttackComponent _asbp_top_down_character) (Variables|Default|GetAmountOfDamage)))

(event Custom|MoveSpeed_Event
  (bind _asbp_top_down_character (Utilities|Casting|CastToBP_TopDownCharacter (Game|GetPlayerCharacter 0)))
  (Default|PlayerSpeedUpgrade _asbp_top_down_character (Variables|Default|GetAmountOfMoveSpeed)))

(event Custom|ProjectileSpeed_Event
  (bind _asbp_top_down_character (Utilities|Casting|CastToBP_TopDownCharacter (Game|GetPlayerCharacter 0)))
  (Default|SpeedUpgrade (Variables|/Game/TopDown/Blueprints/BP_TopDownCharacter.BP_TopDownCharacter_C|GetBPC_AttackComponent _asbp_top_down_character) (Variables|Default|GetAmountOfMoveSpeed)))

(event EventBeginPlay)

(event Collision|EventActorBeginOverlap
  (params (OtherActor :type Actor%20Object%20Reference)))

(event EventTick
  (params (DeltaSeconds :type Float%20%28single-precision%29)))

(fn ConstructionScript)

(fn SetAmountstoZero
  (Variables|Default|SetAmountOfMaxHealth 0.0)
  (Variables|Default|SetAmountOfDamage 0.0)
  (Variables|Default|SetAmountOfMoveSpeed 0.0)
  (Variables|Default|SetAmountOfProjectileSpeed 0.0))